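; BP_ButtonStart is an interactable prop button that acts as a non-working start button, pointing the player toward another button.
; On BeginPlay it binds Press to its interaction event.
; Pressing launches its physics mesh along the player camera's forward vector, then shows a timed sequence of three messages on a console, separated by delays, saying nothing works.
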(event `self.ReceiveBeginPlay`
  (add `self.OnInteraction` (delegate `Press`)))

(event `Press` :!signature `self.OnInteraction`
  (params (InteractingPawn :type "Pawn Object Reference"))
  (`PrimitiveComponent.SetPhysicsLinearVelocity` (`self.Mesh`) (* (`self.GetActorForwardVector` (`GameplayStatics.GetPlayerCameraManager` 0)) 600.0) false "None")
  (bind _console (`/Game/Base/Blueprints/BP_Helpers.GetConsole`))
  (`TextBlock.SetText` _console "This doesn't work!")
  (`KismetSystemLibrary.Delay` 2.0)
  (`TextBlock.SetText` _console "Nothing works here!")
  (`KismetSystemLibrary.Delay` 2.0)
  (`TextBlock.SetText` _console "You should try the other button"))

(fn `UserConstructionScript`
  (`parent.UserConstructionScript`))