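; Control panel prop that lets a player toggle collision and gravity on a referenced Actor through two buttons.
; On BeginPlay, if the Actor is valid, it displays the object's name and binds to each button's interaction event, reaching the buttons through their child component's owner.
; Each press flips the actor's collision, or gravity on its first found primitive component, then updates that button's ON/OFF label.
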(event `self.ReceiveBeginPlay`
  ;[1 1 1] Check for valid actor
  (`/Engine/EditorBlueprintResources/StandardMacros.IsValid` (`self.Actor`)
    (:`Is Valid`
      (`|ExecutionSequence`
        (:`then_0`
          ;[1 1 1] Object name
          (`TextRenderComponent.K2_SetText` (`self.Label_Object`) (`KismetTextLibrary.Conv_StringToText` (`KismetStringLibrary.Concat_StrStr` "Object: " (`KismetSystemLibrary.GetDisplayName` (`self.Actor`))))))
        (:`then_1`
          ;[1 1 1] Toggle collision button
          (bind _asbp_button_toggle_collision (cast `/Game/Environment/Props/Blueprints/BP_ButtonToggleCollision` (`ActorComponent.GetOwner` (`SceneComponent.GetChildComponent` (`self.Button_ToggleCollision`) 0))))
          (add `InteractiveActor.OnInteraction` _asbp_button_toggle_collision (delegate `ChangeCollision`)))
        (:`then_2`
          ;[1 1 1] Toggle gravity button
          (bind _asbp_button_toggle_gravity (cast `/Game/Environment/Props/Blueprints/BP_ButtonToggleGravity` (`ActorComponent.GetOwner` (`SceneComponent.GetChildComponent` (`self.Button_ToggleGravity`) 0))))
          (add `InteractiveActor.OnInteraction` _asbp_button_toggle_gravity (delegate `ChangeGravity`)))))))

(event `ChangeCollision`
  (params (InteractingPawn :type "Pawn Object Reference"))
  ;[1 1 1] Toggle collision button
  (`self.ToggleActorCollision` (stale `self.ReceiveBeginPlay` _asbp_button_toggle_collision)))

(event `ChangeGravity`
  (params (InteractingPawn :type "Pawn Object Reference"))
  ;[1 1 1] Toggle gravity button
  (`self.ToggleActorGravity` (stale `self.ReceiveBeginPlay` _asbp_button_toggle_gravity)))

(fn `ToggleActorCollision`
  (params (Button :type "/Game/Environment/Props/Blueprints/BP_ButtonToggleCollision Object Reference"))
  (bind _actor (`self.Actor`))
  (bind _label (`/Game/Environment/Props/Blueprints/BP_Button.Label` Button))
  (bind _returnvalue (not (`self.GetActorEnableCollision` _actor)))
  (`self.SetActorEnableCollision` _actor _returnvalue)
  (if _returnvalue
    (`TextRenderComponent.K2_SetText` _label "Collision OFF")
    (else
      (`TextRenderComponent.K2_SetText` _label "Collision ON"))))

(fn `ToggleActorGravity`
  (params (Button :type "/Game/Environment/Props/Blueprints/BP_ButtonToggleGravity Object Reference"))
  (bind _label (`/Game/Environment/Props/Blueprints/BP_Button.Label` Button))
  (bind _returnvalue (`self.GetComponentByClass` (`self.Actor`) "/Script/Engine.PrimitiveComponent"))
  (bind _returnvalue_2 (not (`PrimitiveComponent.IsGravityEnabled` _returnvalue)))
  (`PrimitiveComponent.SetEnableGravity` _returnvalue _returnvalue_2)
  (if _returnvalue_2
    (`TextRenderComponent.K2_SetText` _label "Gravity OFF")
    (else
      (`TextRenderComponent.K2_SetText` _label "Gravity ON"))))

(fn `UserConstructionScript`)