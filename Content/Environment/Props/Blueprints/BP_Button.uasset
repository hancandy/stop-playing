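; BP_Button is a button prop that lights up or darkens to show whether it is enabled.
; On BeginPlay it creates a dynamic material instance for the Cube mesh and binds its Toggle event to the OnToggle dispatcher.
; Toggle switches the material's Glow scalar parameter between lit and off according to IsEnabled.
; The graph contains no input or interaction logic, only this visual response.
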(event `self.ReceiveBeginPlay`
  (`|ExecutionSequence`
    (:`then_0`
      (bind _returnvalue (`PrimitiveComponent.CreateDynamicMaterialInstance` (`self.Cube`) 0 (`PrimitiveComponent.GetMaterial` (`self.Cube`) 0)))
      (bind _output_get (set `self.DynamicMaterial` _returnvalue))
      (`PrimitiveComponent.SetMaterial` (`self.Cube`) 0 _output_get))
    (:`then_1`
      (add `self.OnToggle` (delegate `Toggle`)))))

(event `Toggle` :!signature `self.OnToggle`
  (params (bIsEnabled :type Boolean))
  (bind _dynamicmaterial (`self.DynamicMaterial`))
  (if bIsEnabled
    (`MaterialInstanceDynamic.SetScalarParameterValue` _dynamicmaterial "Glow" 4.0)
    (else
      (`MaterialInstanceDynamic.SetScalarParameterValue` _dynamicmaterial "Glow" 0.0))))

(fn `UserConstructionScript`
  (`parent.UserConstructionScript`))