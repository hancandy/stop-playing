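; Basketball prop Blueprint whose material glow switches on and off through a toggle event.
; On BeginPlay it creates a dynamic material instance from the mesh's first material slot, applies it, and binds Toggle to the OnToggle dispatcher.
; The Toggle handler drives the Glow scalar parameter according to the enabled state, while the construction script only calls its parent.
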(event `self.ReceiveBeginPlay`
  (bind _mesh (`self.Mesh`))
  (bind _returnvalue (`PrimitiveComponent.CreateDynamicMaterialInstance` _mesh 0 (`PrimitiveComponent.GetMaterial` _mesh 0)))
  (`PrimitiveComponent.SetMaterial` _mesh 0 _returnvalue)
  (add `self.OnToggle` (delegate `Toggle`)))

(event `Toggle` :!signature `self.OnToggle`
  (params (bIsEnabled :type Boolean))
  (if bIsEnabled
    (`MaterialInstanceDynamic.SetScalarParameterValue` (stale `self.ReceiveBeginPlay` _returnvalue) "Glow" 4.0)
    (else
      (`MaterialInstanceDynamic.SetScalarParameterValue` (stale `self.ReceiveBeginPlay` _returnvalue) "Glow" 0.0))))

(fn `UserConstructionScript`
  (`parent.UserConstructionScript`))