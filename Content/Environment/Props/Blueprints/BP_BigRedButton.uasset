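; BP_BigRedButton is a prop button that removes a referenced DisableActor when an InteractiveActor overlaps it.
; The overlap hides that actor, turns off its collision and plays confirm and door-opening sounds at its location.
; A timeline then slides the button along local Y and drives the Glow parameter on a dynamic material created at BeginPlay.
; Nothing in the graph reverses the effect.
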(event `self.ReceiveBeginPlay`
  (bind _button (`self.Button`))
  (bind _returnvalue (`KismetMaterialLibrary.CreateDynamicMaterialInstance` (`PrimitiveComponent.GetMaterial` _button 0)))
  (`PrimitiveComponent.SetMaterial` _button 0 _returnvalue))

(event `self.ReceiveActorBeginOverlap`
  (params (OtherActor :type "Actor Object Reference"))
  (bind _button (`self.Button`))
  (bind _disableactor (`self.DisableActor`))
  (cast `InteractiveActor` OtherActor)
  (`/Engine/EditorBlueprintResources/StandardMacros.IsValid` _disableactor
    (:`Is Valid`
      (`self.SetActorHiddenInGame` _disableactor true)
      (`self.SetActorEnableCollision` _disableactor false)
      (`GameplayStatics.PlaySoundAtLocation` "/Game/Base/Sounds/S_ButtonConfirm.S_ButtonConfirm" (`self.K2_GetActorLocation` _disableactor))
      ;[1 1 1] Actor sound
      (`GameplayStatics.PlaySoundAtLocation` "/Game/Base/Sounds/S_OpenDoor.S_OpenDoor" (`self.K2_GetActorLocation` (`self.DisableActor`)))
      ;[1 1 1] Button sound
      (`GameplayStatics.PlaySoundAtLocation` null (`self.K2_GetActorLocation`))
      (bind (_direction _amount _glow) (`Timeline|Button Animation`)
        (:`Update`
          (`SceneComponent.K2_SetRelativeLocation` _button (`KismetMathLibrary.MakeVector` 0.0 _amount) false false)
          (bind _asmaterial_instance_dynamic (cast `MaterialInstanceDynamic` (`PrimitiveComponent.GetMaterial` _button 0)))
          (`MaterialInstanceDynamic.SetScalarParameterValue` _asmaterial_instance_dynamic "Glow" _glow))))
    (:`Is Not Valid`
      (`KismetSystemLibrary.PrintString` "DisabeActor not vaid"))))

(fn `UserConstructionScript`)