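; Player character Blueprint that creates the HUD, shows interaction prompts, plays grab and release sounds, and reloads the level on R.
; BeginPlay creates the HUD and binds the interaction, grab, release and gravity-scale events.
; When a gravity-scale change requires a flip, a timeline incrementally rotates Ninja movement's gravity around Y, then snaps it to vertical.
; Capsule collision is disabled during the flip.
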(event `Key|R`
  (params (Key :type "Key Structure" :default "AnyKey"))
  ;[1 1 1] Reset level
  (:`Pressed`
    (bind _returnvalue (`GameplayStatics.GetCurrentLevelName` true))
    (`GameplayStatics.OpenLevel` (`KismetStringLibrary.Conv_StringToName` _returnvalue))))

(event `self.ReceiveBeginPlay`
  (`|ExecutionSequence`
    (:`then_0`
      (`self.InitHUD`))
    (:`then_1`
      (add `self.OnInteractionPrompt` (delegate `InteractionPrompt`)))
    (:`then_2`
      (add `self.OnGrabActor` (delegate `GrabActor`))
      (add `self.OnReleaseActor` (delegate `ReleaseActor`)))
    (:`then_3`
      ;[1 1 1] Gravity scale
      (add `self.OnSetGravityScale` (delegate `SetGravityScale`)))))

(event `InteractionPrompt` :!signature `self.OnInteractionPrompt`
  (params (Message :type String))
  (`self.ShowInteractionPrompt` Message))

(event `GrabActor`
  (`self.PlayGrabSound`))

(event `ReleaseActor`
  (`self.PlayReleaseSound`))

(event `SetGravityScale` :!signature `self.OnSetGravityScale`
  (params (NewGravityScale :type "Float (double-precision)"))
  ;[1 1 1] Gravity scale
  (bind (_bshouldrotategravity _ninjamovement) (`self.ShouldRotateGravity` NewGravityScale))
  (if _bshouldrotategravity
    (`PrimitiveComponent.SetCollisionEnabled` (`self.CapsuleComponent`) "NoCollision")
    (bind (_direction _amount) (`Timeline|GravityTimeline` :!via `PlayFromStart`)
      (:`Update`
        (`NinjaCharacterMovementComponent.SetGravityDirection` _ninjamovement (`KismetMathLibrary.RotateAngleAxis` (`NinjaCharacterMovementComponent.GetGravityDirection` _ninjamovement false) (* _amount 2.95) (0.0 1.0 0.0))))
      (:`Finished`
        (`PrimitiveComponent.SetCollisionEnabled` (`self.CapsuleComponent`) "QueryAndPhysics")
        (`NinjaCharacterMovementComponent.SetGravityDirection` _ninjamovement (`KismetMathLibrary.MakeVector` 0.0 0.0 (* NewGravityScale -1.0)))))))

(fn `ShouldRotateGravity`
  (params (NewGravityDirection :type "Float (double-precision)"))
  (returns (bShouldRotateGravity :type Boolean) (NinjaMovement :type "NinjaCharacterMovementComponent Object Reference"))
  (locals (bShouldRotate :type Boolean))
  (bind _asninja_character_movement_component (cast `NinjaCharacterMovementComponent` (`self.CharacterMovement`))
    (:`then`
      _)
    (:`CastFailed`
      _))
  (bind _output_get (set `local.bShouldRotate` (> (* NewGravityDirection (.z (`NinjaCharacterMovementComponent.GetGravityDirection` _asninja_character_movement_component false))) 0.0)))
  (return _output_get _asninja_character_movement_component))

(fn `UserConstructionScript`)